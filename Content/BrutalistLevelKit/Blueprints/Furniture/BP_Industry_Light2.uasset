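; BP_Industry_Light2 is a placeable industrial light fixture with a furniture mesh and a spot light, set up entirely in the construction script.
; It is either switched by the Active flag or, when Random is set, by a seeded 50/50 roll from a random stream.
; The result toggles spot light visibility and drives the emissive color of a dynamic material on the mesh, black when off, with Color tinting both.
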(event EventBeginPlay
  (|CallParentFunction) ; This node is disabled and will not be called.\nDrag off pins to build functionality.
)

(event Collision|EventActorBeginOverlap
  (params (OtherActor :type Actor%20Object%20Reference))
  (|CallParentFunction OtherActor) ; This node is disabled and will not be called.\nDrag off pins to build functionality.
)

(event EventTick
  (params (DeltaSeconds :type Float%20%28single-precision%29))
  (|CallParentFunction DeltaSeconds) ; This node is disabled and will not be called.\nDrag off pins to build functionality.
)

(fn ConstructionScript
  (bind _furnituremesh (Variables|Default|GetFurnitureMesh))
  (bind _color (Variables|Default|GetColor))
  (bind _spotlight (Variables|Default|GetSpotLight))
  (|CallParentFunction)
  (LocalVariables|SetLocalRandom (select (Variables|Control|GetRandom) (Class|KismetMathLibrary|RandomBoolwithWeightfromStream 0.5 (Variables|Default|GetRandomSeedStruct)) (Variables|Default|GetActive)))
  (bind _returnvalue (Rendering|Material|CreateDynamicMaterialInstance _furnituremesh 0 (Rendering|Material|GetMaterial _furnituremesh 0) "None" :!class /Script/Engine.PrimitiveComponent))
  (bind _output_get (Variables|Control|SetLightMatInst _returnvalue))
  (Rendering|Material|SetVectorParameterValue _output_get "EmissiveColor" (select (LocalVariables|GetLocalRandom) _color "") :!class /Script/Engine.MaterialInstanceDynamic)
  (Rendering|SetVisibility _spotlight (LocalVariables|GetLocalRandom) false)
  (Rendering|Components|Light|SetLightColor _spotlight _color true))