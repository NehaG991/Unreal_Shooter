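; Melee enemy pawn that feeds perception and patrol data into the blackboard of its EnemyController_BP AI controller.
; On BeginPlay it caches the controller and writes two patrol points as offsets from its spawn location.
; An aggro sphere sets or clears TargetActor, and an attack sphere toggles InAttackRange, as the MainCharacter enters or leaves.
; Overlap handlers re-fetch the controller if the cached reference is invalid.
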(event OnComponentBeginOverlap(AgroSphere)
  (params (OverlappedComponent :type Primitive%20Component%20Object%20Reference) (OtherActor :type Actor%20Object%20Reference) (OtherComp :type Primitive%20Component%20Object%20Reference) (OtherBodyIndex :type Integer) (bFromSweep :type Boolean) (SweepResult :type Hit%20Result%20Structure%20%28by%20ref%29))
  ;[1 0 0.8111] Agrosphere Collision
  (Utilities|IsValid OtherActor
    (:Is%20Valid
      (bind _asmain_character (Utilities|Casting|CastToMainCharacter OtherActor))
      (Utilities|IsValid _asmain_character
        (:Is%20Valid
          (Utilities|IsValid (Variables|Default|GetEnemyController)
            (:Is%20Valid
              _)
            (:Is%20Not%20Valid
              (bind _asenemy_controller_bp (Utilities|Casting|CastToEnemyController_BP (Pawn|GetController)))
              (Variables|Default|SetEnemyController _asenemy_controller_bp)))
          (AI|Components|Blackboard|SetValueasObject (AI|GetBlackboard (Variables|Default|GetEnemyController)) (Utilities|Name|MakeLiteralName "TargetActor") _asmain_character))))))

(event OnComponentEndOverlap(AgroSphere)
  (params (OverlappedComponent :type Primitive%20Component%20Object%20Reference) (OtherActor :type Actor%20Object%20Reference) (OtherComp :type Primitive%20Component%20Object%20Reference) (OtherBodyIndex :type Integer))
  ;[1 0 0.8111] Agrosphere Collision
  (Utilities|IsValid OtherActor
    (:Is%20Valid
      (bind _asmain_character (Utilities|Casting|CastToMainCharacter OtherActor))
      (Utilities|IsValid _asmain_character
        (:Is%20Valid
          (Utilities|IsValid (Variables|Default|GetEnemyController)
            (:Is%20Valid
              _)
            (:Is%20Not%20Valid
              (bind _asenemy_controller_bp (Utilities|Casting|CastToEnemyController_BP (Pawn|GetController)))
              (Variables|Default|SetEnemyController _asenemy_controller_bp)))
          (AI|Components|Blackboard|SetValueasObject (AI|GetBlackboard (Variables|Default|GetEnemyController)) (Utilities|Name|MakeLiteralName "TargetActor") 0))))))

(event OnComponentBeginOverlap(AttackSphere)
  (params (OverlappedComponent :type Primitive%20Component%20Object%20Reference) (OtherActor :type Actor%20Object%20Reference) (OtherComp :type Primitive%20Component%20Object%20Reference) (OtherBodyIndex :type Integer) (bFromSweep :type Boolean) (SweepResult :type Hit%20Result%20Structure%20%28by%20ref%29))
  ;[1 0 0.8111] Attack Sphere Collision
  (Utilities|IsValid OtherActor
    (:Is%20Valid
      (bind _asmain_character (Utilities|Casting|CastToMainCharacter OtherActor))
      (Utilities|IsValid _asmain_character
        (:Is%20Valid
          (Utilities|IsValid (Variables|Default|GetEnemyController)
            (:Is%20Valid
              _)
            (:Is%20Not%20Valid
              (bind _asenemy_controller_bp (Utilities|Casting|CastToEnemyController_BP (Pawn|GetController)))
              (Variables|Default|SetEnemyController _asenemy_controller_bp)))
          (AI|Components|Blackboard|SetValueasBool (AI|GetBlackboard (Variables|Default|GetEnemyController)) (Utilities|Name|MakeLiteralName "InAttackRange") true))))))

(event OnComponentEndOverlap(AttackSphere)
  (params (OverlappedComponent :type Primitive%20Component%20Object%20Reference) (OtherActor :type Actor%20Object%20Reference) (OtherComp :type Primitive%20Component%20Object%20Reference) (OtherBodyIndex :type Integer))
  ;[1 0 0.8111] Attack Sphere Collision
  (Utilities|IsValid OtherActor
    (:Is%20Valid
      (bind _asmain_character (Utilities|Casting|CastToMainCharacter OtherActor))
      (Utilities|IsValid _asmain_character
        (:Is%20Valid
          (Utilities|IsValid (Variables|Default|GetEnemyController)
            (:Is%20Valid
              _)
            (:Is%20Not%20Valid
              (bind _asenemy_controller_bp (Utilities|Casting|CastToEnemyController_BP (Pawn|GetController)))
              (Variables|Default|SetEnemyController _asenemy_controller_bp)))
          (AI|Components|Blackboard|SetValueasBool (AI|GetBlackboard (Variables|Default|GetEnemyController)) (Utilities|Name|MakeLiteralName "InAttackRange") false))))))

(event EventBeginPlay
  (bind _asenemy_controller_bp (Utilities|Casting|CastToEnemyController_BP (Pawn|GetController)))
  (Variables|Default|SetEnemyController _asenemy_controller_bp)
  ;[1 1 1] Setting Patrol Points
  (AI|Components|Blackboard|SetValueasVector (AI|GetBlackboard (Variables|Default|GetEnemyController)) (Utilities|Name|MakeLiteralName "PatrolPoint1") (+ (Variables|Default|GetPatrolPoint1) (Transformation|GetActorLocation)))
  (AI|Components|Blackboard|SetValueasVector (AI|GetBlackboard (Variables|Default|GetEnemyController)) (Utilities|Name|MakeLiteralName "PatrolPoint2") (+ (Variables|Default|GetPatrolPoint2) (Transformation|GetActorLocation))))

(fn ConstructionScript)