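; Player character Blueprint for a shooter, handling aim zoom, sprint, crouch, shooting and reloading.
; Tick polls right mouse to swap HUD crosshairs, limit sprinting and update MainAnim_BP; sprint and crouch adjust walk speed, crouch also lowering the camera boom.
; Shooting, blocked while sprinting or reloading, traces along camera forward to orient a spawned Bullet_BP, adding muzzle effects and hip or ironsight montages.
; Reload refills the seven-round magazine from held ammo.
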(event Custom|Toggle%20Zoom
  ;[1 1 1] Toggles Between Zoom and Default Crosshairs if RMB is Held Down
  (if (Game|Player|IsInputKeyDown (Game|GetPlayerController 0) "RightMouseButton")
    (bind _foundwidgets (Widget|GetAllWidgetsOfClass "/Game/Blueprints/HUDOverlayWidget.HUDOverlayWidget_C" true))
    (Default|ToggleZoomCrosshair _foundwidgets)
    (Variables|Default|SetZooming true)
    ;;[1 1 1] Resets Sprint to Normal Walk
    (Variables|/Script/Engine.CharacterMovementComponent|SetMaxWalkSpeed (Variables|Character|GetCharacterMovement) 5e+02)
    (else
      (bind _foundwidgets_2 (Widget|GetAllWidgetsOfClass "/Game/Blueprints/HUDOverlayWidget.HUDOverlayWidget_C" true))
      (Default|ToggleDefaultCrosshair _foundwidgets_2)
      (Variables|Default|SetZooming false)
      (if (Variables|Default|GetIsSprinting)
        (Variables|/Script/Engine.CharacterMovementComponent|SetMaxWalkSpeed (Variables|Character|GetCharacterMovement) 7.5e+02))))
  (bind _asmain_anim_bp (Utilities|Casting|CastToMainAnim_BP (Components|SkeletalMesh|GetAnimInstance (Variables|Character|GetMesh))))
  (Variables|/Game/Sci_Fi_Character_08/Animations/MainAnim_BP.MainAnim_BP_C|SetIsZoomed _asmain_anim_bp (Variables|Default|GetZooming)))

(event EventBeginPlay)

(event Collision|EventActorBeginOverlap
  (params (OtherActor :type Actor%20Object%20Reference)))

(event EventTick
  (params (DeltaSeconds :type Float%20%28single-precision%29))
  (CallFunction|ToggleZoom))

(event Input|ActionEvents|InputActionShoot
  (params (Key :type Key%20Structure :default "None"))
  (bind _bullet_startpoint (Variables|Default|GetBullet%20StartPoint))
  (bind _bullet_startpoint_2 (Variables|Default|GetBullet%20StartPoint))
  (bind _returnvalue (Transformation|GetWorldLocation _bullet_startpoint))
  (bind _returnvalue_2 (Transformation|GetWorldLocation _bullet_startpoint_2))
  ;[1 1 1] Shooting Functiaonlity
  ;;[1 1 1] Can only fire if NOT spriting AND NOT reloading
  (:Pressed
    (bind _asmain_anim_bp (Utilities|Casting|CastToMainAnim_BP (Components|SkeletalMesh|GetAnimInstance (Variables|Character|GetMesh))))
    (if (and (not (Variables|Default|GetIsSprinting)) (not (Variables|/Game/Sci_Fi_Character_08/Animations/MainAnim_BP.MainAnim_BP_C|GetIsReloading _asmain_anim_bp)))
      ;;[1 1 1] Decreases Current Ammo
      (if (> (Variables|Default|GetCurrent%20Ammo) 0)
        (Variables|Default|SetCurrent%20Ammo (- (Variables|Default|GetCurrent%20Ammo) 1))
        (Variables|Default|SetShooting true)
        (bind (_outhit _returnvalue_3) (Collision|LineTraceByChannel _returnvalue (+ _returnvalue (* (Math|Vector|GetForwardVector (Variables|Default|GetFollowCamera)) 1e+04)) "TraceTypeQuery1" false 0 "None"))
        (Game|SpawnActorfromClass "/Game/Blueprints/Bullet_BP.Bullet_BP_C" (Math|Transform|MakeTransform _returnvalue_2 (Math|Rotator|FindLookatRotation _returnvalue_2 (Math|Vector|SelectVector (.ImpactPoint (Collision|BreakHitResult _outhit)) (.TraceEnd (Collision|BreakHitResult _outhit)) _returnvalue_3)) "0.200000,0.200000,0.200000") "Undefined" 0 0)
        (Effects|SpawnEmitterAttached "/Game/InfinityBladeEffects/Effects/FX_Monsters/FX_Monster_Gruntling/FlameThrower/P_FlameExplode.P_FlameExplode" (Variables|Default|GetBullet%20StartPoint) "None" _returnvalue_2 (Math|Rotator|FindLookatRotation _returnvalue_2 (Math|Vector|SelectVector (.ImpactPoint (Collision|BreakHitResult _outhit)) (.TraceEnd (Collision|BreakHitResult _outhit)) _returnvalue_3)) "0.030000,0.030000,0.030000" "KeepWorldPosition")
        (if (Variables|Default|GetZooming)
          (Animation|PlayAnimMontage "/Game/Sci_Fi_Character_08/Animations/Fire_Ironsight_Montage.Fire_Ironsight_Montage" 1.0 "None")
          (else
            (Animation|PlayAnimMontage "/Game/Sci_Fi_Character_08/Animations/Fire_Hip_Montage.Fire_Hip_Montage" 1.0 "None")))
        (bind _asmain_anim_bp_2 (Utilities|Casting|CastToMainAnim_BP (Components|SkeletalMesh|GetAnimInstance (Variables|Character|GetMesh)) :!label _label))
        (Variables|/Game/Sci_Fi_Character_08/Animations/MainAnim_BP.MainAnim_BP_C|SetIsShooting _asmain_anim_bp_2 (Variables|Default|GetShooting)))))
  (:Released
    (Variables|Default|SetShooting false)
    (goto _label)))

(event Input|ActionEvents|InputActionSprint
  (params (Key :type Key%20Structure :default "None"))
  (bind _charactermovement (Variables|Character|GetCharacterMovement))
  ;[1 1 1] Sprint Functionality - Can't sprint if zoomed it
  (:Pressed
    (Variables|Default|SetIsSprinting true)
    (if (not (Variables|Default|GetZooming))
      (Variables|/Script/Engine.CharacterMovementComponent|SetMaxWalkSpeed _charactermovement 7.5e+02)))
  (:Released
    (Variables|Default|SetIsSprinting false)
    (Variables|/Script/Engine.CharacterMovementComponent|SetMaxWalkSpeed _charactermovement 5e+02)))

(event Input|ActionEvents|InputActionCrouch
  (params (Key :type Key%20Structure :default "None"))
  (bind _cameraboom (Variables|Default|GetCameraboom))
  (bind _charactermovement (Variables|Character|GetCharacterMovement))
  ;[1 1 1] Crouch Functionality
  (:Pressed
    (Variables|Default|SetIsCrouching true)
    (Variables|/Script/Engine.CharacterMovementComponent|SetMaxWalkSpeed _charactermovement 2.5e+02)
    (Transformation|SetRelativeLocation _cameraboom "0, 0,30.000000" false false))
  (:Released
    (Variables|Default|SetIsCrouching false)
    (Variables|/Script/Engine.CharacterMovementComponent|SetMaxWalkSpeed _charactermovement 5e+02)
    (Transformation|SetRelativeLocation _cameraboom "0, 0,75.000000" false false)))

(event Input|ActionEvents|InputActionReload
  (params (Key :type Key%20Structure :default "None"))
  ;[1 1 1] Reloading Functionality
  (:Pressed
    ;;[1 1 1] Can't Reload if Curr Ammo is 7 OR Held is 0
    (if (not (or (== (Variables|Default|GetCurrent%20Ammo) 7) (== (Variables|Default|GetHeld%20Ammo) 0)))
      (Animation|PlayAnimMontage "/Game/Sci_Fi_Character_08/Animations/Reload_Montage.Reload_Montage" 1.0 "None")
      (if (>= (- (Variables|Default|GetHeld%20Ammo) (- 7 (Variables|Default|GetCurrent%20Ammo))) 0)
        (Variables|Default|SetHeld%20Ammo (- (Variables|Default|GetHeld%20Ammo) (- 7 (Variables|Default|GetCurrent%20Ammo))))
        (Variables|Default|SetCurrent%20Ammo 7)
        (else
          (Variables|Default|SetCurrent%20Ammo (+ (Variables|Default|GetCurrent%20Ammo) (Variables|Default|GetHeld%20Ammo)))
          (Variables|Default|SetHeld%20Ammo 0))))))

(fn ConstructionScript)