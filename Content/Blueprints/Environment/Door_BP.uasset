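; Interactable door Blueprint that slides a door component vertically to open and close.
; Interact plays the Timeline from the start when Closed is true and reverses it from the end otherwise, printing that flag for debugging.
; The DoorOpening track drives the door's relative Z location, and the Closed flag flips only when the Timeline finishes.
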(event Custom|Interact
  (Development|PrintString (Utilities|String|ToString(Boolean) (Variables|Default|GetClosed)))
  (if (Variables|Default|GetClosed)
    (bind _door_opening (Timeline|Timeline PlayFromStart)
      (:Update
        (Transformation|SetRelativeLocation (Variables|Default|GetDoor) (Math|Vector|MakeVector 0.0 0.0 _door_opening) false false))
      (:Finished
        (Variables|Default|SetClosed (not (Variables|Default|GetClosed)))))
    (else
      (Timeline|Timeline ReverseFromEnd))))

(event EventBeginPlay
  (Variables|Default|SetClosed true))

(event Collision|EventActorBeginOverlap
  (params (OtherActor :type Actor%20Object%20Reference)))

(event EventTick
  (params (DeltaSeconds :type Float%20%28single-precision%29)))

(fn ConstructionScript)